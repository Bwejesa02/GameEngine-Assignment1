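; BP_WallFactory is the wall variant in a factory pattern, overriding a parent's CreateObstacle to spawn a BP_Wall actor.
; CreateObstacle spawns the wall at the world origin with zero rotation and unit scale.
; Its parent call and return node are disconnected, so the spawned wall never reaches the return node.
; The event graph holds only disabled default events, and the construction script just calls its parent.
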(fn `CreateObstacle`
  (returns (NewParam :type "Actor Object Reference"))
  (bind _returnvalue (`|SpawnActorFromClass` "/Game/Blueprints/BP_Wall.BP_Wall_C" (`KismetMathLibrary.MakeTransform` (0.0 0.0 0.0)) "Undefined" "MultiplyWithRoot" null null)))

(fn `UserConstructionScript`
  (`parent.UserConstructionScript`))